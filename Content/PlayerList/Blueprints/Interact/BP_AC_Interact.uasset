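; BP_AC_Interact is an actor component that gives its owning actor an interaction decal, hidden by default.
; On BeginPlay it creates a dynamic instance of MAT_Decal_Interact and spawns a rotated decal attached to the owner's root component, each only if not already valid.
; A helper function toggles the decal's visibility, and optional debug messages trace the setup steps.
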(event Custom|EventACInteractInitDecal
  (Utilities|FlowControl|Sequence
    (:then_0
      (CallFunction|FuncShowDebugMessage (Variables|DEBUG|GetbShowDebug) "BP_AC_Interact - Event Decal Init"))
    (:then_1
      (Variables|Default|GetAs%20MAT_Decal_Interact
        (:then)
        (:else
          (bind _returnvalue (Rendering|Material|CreateDynamicMaterialInstance "/Game/PlayerList/Blueprints/Interact/Material/MAT_Decal_Interact.MAT_Decal_Interact" "None" "None" :!class /Script/Engine.KismetMaterialLibrary))
          (Variables|Default|SetAs%20MAT_Decal_Interact _returnvalue))))
    (:then_2
      (Variables|Default|GetAs%20Decal_Interact
        (:then
          _)
        (:else
          (bind _returnvalue_2 (Class|GameplayStatics|SpawnDecalAttached (Variables|Default|GetAs%20MAT_Decal_Interact) "0, 0, 0" (Variables|/Script/Engine.Actor|GetRootComponent (Components|GetOwner)) "None" "0, 0, 0" "-90.000000,0.000000,0.000000" "KeepRelativeOffset" 0.0))
          (Variables|Default|SetAs%20Decal_Interact _returnvalue_2)))
      (CallFunction|FuncUpdateDecalVisibility false))))

(event EventBeginPlay
  (Utilities|FlowControl|Sequence
    (:then_0
      (CallFunction|FuncShowDebugMessage (Variables|DEBUG|GetbShowDebug) "BP_AC_Interact - Event Begin Play"))
    (:then_1
      (CallFunction|EventACInteractInitDecal))))

(event EventTick
  (params (DeltaSeconds :type Float%20%28single-precision%29)))

(fn FuncUpdateDecalVisibility
  (params (bNewVisibility :type Boolean))
  (Rendering|SetVisibility (Variables|Default|GetAs%20Decal_Interact) bNewVisibility false))