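; Actor component that stores its owner's team and marks the owner with a team decal on the ground.
; On BeginPlay it creates a dynamic decal material and spawns it attached to the root at the base of the owner's bounds, sized from them.
; A helper tints the decal by team, but init calls it before the decal spawns and the team setter does not call it.
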(event Custom|EventACTeamInitDecal
  (bind _returnvalue (Components|GetOwner))
  (bind _boxextent (Collision|GetActorBounds _returnvalue false false))
  (Utilities|FlowControl|Sequence
    (:then_0
      (CallFunction|FuncShowDebugMessage (Variables|DEBUG|GetbShowDebug) "BP_AC_Team - Event Decal Init"))
    (:then_1
      (Variables|Material|GetAs%20MAT_Decal_Team
        (:then
          _)
        (:else
          (bind _returnvalue_2 (Rendering|Material|CreateDynamicMaterialInstance "/Game/PlayerList/Blueprints/Team/Material/MAT_Decal_Team.MAT_Decal_Team" "None" "None" :!class /Script/Engine.KismetMaterialLibrary))
          (Variables|Material|SetAs%20MAT_Decal_Team _returnvalue_2)))
      (CallFunction|FuncUpdateMaterialColor))
    (:then_2
      (Variables|Default|GetAs%20Decal_Team
        (:then)
        (:else
          (bind _returnvalue_3 (Class|GameplayStatics|SpawnDecalAttached (Variables|Material|GetAs%20MAT_Decal_Team) (+ _boxextent 5.0) (Variables|/Script/Engine.Actor|GetRootComponent _returnvalue) "None" (- (Transformation|GetActorLocation _returnvalue) (Math|Vector|MakeVector 0.0 0.0 (.Z (Math|Vector|BreakVector _boxextent)))) (Math|Conversions|RotationFromXVector (Transformation|GetActorUpVector _returnvalue)) "KeepRelativeOffset" 0.0))
          (Variables|Default|SetAs%20Decal_Team _returnvalue_3))))))

(event EventBeginPlay
  (Utilities|FlowControl|Sequence
    (:then_0
      (CallFunction|FuncShowDebugMessage (Variables|DEBUG|GetbShowDebug) "BP_AC_Team - Event Begin Play"))
    (:then_1
      (CallFunction|EventACTeamInitDecal))))

(event EventTick
  (params (DeltaSeconds :type Float%20%28single-precision%29)))

(fn FuncGetTeam
  (return (Variables|Default|GetTeam)))

(fn FuncSetTeam
  (params (Team :type E_Team%20Enum :default "NewEnumerator0"))
  (Variables|Default|SetTeam Team))

(fn FuncUpdateMaterialColor
  (bind _as_decal_team (Variables|Default|GetAs%20Decal_Team)
    (:then
      (Rendering|Components|Decal|SetDecalColor _as_decal_team (Utilities|Select :Index (Variables|Default|GetTeam) :NewEnumerator0 "" :NewEnumerator1 (Variables|Default|GetTeamBlueColor) :NewEnumerator2 (Variables|Default|GetTeamRedColor) :NewEnumerator3 "" :NewEnumerator4 (Variables|Default|GetTeamNeutralColor))))
    (:else)))