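; Gameplay HUD Blueprint that creates and manages the player's on-screen widgets.
; BeginPlay adds the main gameplay widget, sets Game and UI input focused on it, and toggles the debug widget on.
; Events toggle the debug, interact and scoreboard widgets by removing a valid stored instance or creating a new one.
; A separate event forwards the interacted actor to the open interact widget, and optional debug messages trace each event.
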(event Custom|EventHUDWBPDebug
  (Utilities|FlowControl|Sequence
    (:then_0
      (CallFunction|FuncShowDebugMessage (Variables|DEBUG|GetbShowDebug) "BP_HUD_Gameplay - Event WBP Debug"))
    (:then_1
      (bind _as_wbp_hud_gameplay_debug (Variables|DEBUG|GetAs%20WBP_HUD_Gameplay_Debug)
        (:then
          (Widget|RemovefromParent _as_wbp_hud_gameplay_debug)
          (Variables|DEBUG|SetAs%20WBP_HUD_Gameplay_Debug 0))
        (:else
          (bind _returnvalue (UserInterface|CreateWidget "/Game/PlayerList/Gameplay/HUD/UI/DEBUG/WBP_HUD_Debug.WBP_HUD_Debug_C"))
          (bind _output_get (Variables|DEBUG|SetAs%20WBP_HUD_Gameplay_Debug _returnvalue))
          (UserInterface|Viewport|AddtoViewport _output_get 0))))))

(event EventBeginPlay
  (Utilities|FlowControl|Sequence
    (:then_0
      (CallFunction|FuncShowDebugMessage (Variables|DEBUG|GetbShowDebug) "BP_HUD_Gameplay - Event Begin Play")
      (CallFunction|EventHUDWBPDebug))
    (:then_1
      (bind _returnvalue (UserInterface|CreateWidget "/Game/PlayerList/Gameplay/HUD/WB_HUD_Gameplay.WB_HUD_Gameplay_C"))
      (bind _output_get (Variables|Default|SetAs%20WBP_HUD_Gameplay _returnvalue))
      (UserInterface|Viewport|AddtoViewport _output_get 0))
    (:then_2
      (Input|SetInputModeGameandUI (Game|GetPlayerController 0) (Variables|Default|GetAs%20WBP_HUD_Gameplay) "DoNotLock" true false))))

(event EventTick
  (params (DeltaSeconds :type Float%20%28single-precision%29)))

(event Custom|EventHUDInteractUI
  (Utilities|FlowControl|Sequence
    (:then_0
      (CallFunction|FuncShowDebugMessage (Variables|DEBUG|GetbShowDebug) "BP_Character_Unit - Event Interact UI"))
    (:then_1
      (bind _as_wbp_interact (Variables|Interact|GetAs%20WBP_Interact)
        (:then
          (Widget|RemovefromParent _as_wbp_interact)
          (Variables|Interact|SetAs%20WBP_Interact 0))
        (:else
          (bind _returnvalue (UserInterface|CreateWidget "/Game/PlayerList/Blueprints/Interact/UI/WBP_Interact.WBP_Interact_C" 0 0))
          (bind _output_get (Variables|Interact|SetAs%20WBP_Interact _returnvalue))
          (UserInterface|Viewport|AddtoViewport _output_get 0))))))

(event Custom|EventHUDInteractActor
  (params (InteractActor :type BP%20Character%20Unit%20Object%20Reference))
  (Utilities|FlowControl|Sequence
    (:then_0
      (CallFunction|FuncShowDebugMessage (Variables|DEBUG|GetbShowDebug) "BP_Character_Unit - Event Interact Actor"))
    (:then_1
      (bind _as_wbp_interact (Variables|Interact|GetAs%20WBP_Interact)
        (:then
          (Default|EventWBPInteractUpdate _as_wbp_interact InteractActor))
        (:else)))))

(event Custom|EventHUDWBPScoreboard
  (Utilities|FlowControl|Sequence
    (:then_0
      (CallFunction|FuncShowDebugMessage (Variables|DEBUG|GetbShowDebug) "BP_HUD_Gameplay - Event WBP Scoreboard"))
    (:then_2
      (bind _as_wbp_hud_gameplay_scoreboard (Variables|Default|GetAs%20WBP_HUD_Gameplay_Scoreboard)
        (:then
          (Widget|RemovefromParent _as_wbp_hud_gameplay_scoreboard)
          (Variables|Default|SetAs%20WBP_HUD_Gameplay_Scoreboard 0))
        (:else
          (bind _returnvalue (UserInterface|CreateWidget "/Game/PlayerList/Gameplay/HUD/UI/Scoreboard/WB_HUD_Gameplay_Scoreboard.WB_HUD_Gameplay_Scoreboard_C"))
          (bind _output_get (Variables|Default|SetAs%20WBP_HUD_Gameplay_Scoreboard _returnvalue))
          (UserInterface|Viewport|AddtoViewport _output_get 0))))))

(fn ConstructionScript)