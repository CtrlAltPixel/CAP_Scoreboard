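; BP_Character_Unit is a gameplay character that reports its spawn and death to the player controller and game mode.
; On play it blocks a custom trace channel on its capsule and disables mesh decals; possession triggers spawn registration.
; Registration updates BP_PC_Gameplay and notifies a cached BP_GM_Gameplay, with bot registration left unimplemented.
; The death event, not triggered here, clears the controller's unit, notifies the game mode and destroys the actor.
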(event Custom|EventUnitRegisterSpawn
  (Utilities|FlowControl|Sequence
    (:then_0
      (CallFunction|FuncShowDebugMessage (Variables|DEBUG|GetbShowDebug) "BP_Character_Unit - Event Resgister Spawn"))
    (:then_1
      (bind _playercontroller (Variables|Default|GetPlayerController)
        (:then
          (bind _asbp_pc_gameplay (Utilities|Casting|CastToBP_PC_Gameplay _playercontroller))
          (Default|EventPlayerControllerUpdateUnit _asbp_pc_gameplay self))
        (:else
          ;[0.15 0.15 0.15 0.5] register with a bot array in GS, GM or in an actor manager?
          (Utilities|Casting|CastToBP_GS_Gameplay (Game|GetGameState)))))
    (:then_2
      (Variables|Default|GetAs%20BP_GM_Gameplay
        (:then
          _)
        (:else
          (bind _asbp_gm_gameplay (Utilities|Casting|CastToBP_GM_Gameplay (Game|GetGameMode)))
          (Variables|Default|SetAs%20BP_GM_Gameplay _asbp_gm_gameplay)))
      (Default|CallOnUnitSpawn (Variables|Default|GetAs%20BP_GM_Gameplay) self))))

(event Custom|EventUnitRegisterDeath
  (Utilities|FlowControl|Sequence
    (:then_0
      (CallFunction|FuncShowDebugMessage (Variables|DEBUG|GetbShowDebug) "BP_Character_Unit - Event Resgister Death"))
    (:then_1
      (bind _playercontroller (Variables|Default|GetPlayerController)
        (:then
          (bind _asbp_pc_gameplay (Utilities|Casting|CastToBP_PC_Gameplay _playercontroller))
          (Default|EventPlayerControllerUpdateUnit _asbp_pc_gameplay))
        (:else)))
    (:then_2
      (Variables|Default|GetAs%20BP_GM_Gameplay
        (:then
          _)
        (:else
          (bind _asbp_gm_gameplay (Utilities|Casting|CastToBP_GM_Gameplay (Game|GetGameMode)))
          (Variables|Default|SetAs%20BP_GM_Gameplay _asbp_gm_gameplay)))
      (Default|CallOnUnitDeath (Variables|Default|GetAs%20BP_GM_Gameplay) self))
    (:then_3
      (Actor|DestroyActor))))

(event EventBeginPlay
  (Utilities|FlowControl|Sequence
    (:then_0
      (CallFunction|FuncShowDebugMessage (Variables|DEBUG|GetbShowDebug) "BP_Character_Unit - Event Begin Play"))
    (:then_1
      (Collision|SetCollisionResponsetoChannel (Variables|Collision|GetCapsuleComponent) "ECC_GameTraceChannel1" "ECR_Block")
      (Rendering|SetReceivesDecals (Variables|Character|GetMesh) false))))

(event EventPossessed
  (params (NewController :type Controller%20Object%20Reference))
  (Utilities|FlowControl|Sequence
    (:then_0
      (CallFunction|FuncShowDebugMessage (Variables|DEBUG|GetbShowDebug) "BP_Character_Unit - Event Possessed"))
    (:then_1
      (CallFunction|EventUnitRegisterSpawn))))

(fn ConstructionScript)