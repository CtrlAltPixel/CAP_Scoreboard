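; Gameplay player controller that handles camera, click interaction and scoreboard input, and stores the player's unit and loadout.
; On BeginPlay, the local controller caches its HUD and camera pawn, enables the cursor and adds Enhanced Input contexts.
; Camera and scoreboard actions forward to those objects, while primary click traces under the cursor to swap the interacted actor via begin/end messages.
; Missed clicks add a drag context until release, and a debug key kills the selected unit.
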(event Custom|EventDEBUGKillTargetUnit
  (bind _as_bp_actor_interact (Variables|Interact|GetAs%20BP_Actor_Interact)
    (:then
      (bind _asbp_character_unit (Utilities|Casting|CastToBP_Character_Unit _as_bp_actor_interact))
      (Default|EventUnitRegisterDeath _asbp_character_unit))
    (:else)))

(event EventBeginPlay
  (Utilities|FlowControl|Sequence
    (:then_0
      (CallFunction|FuncShowDebugMessage (Variables|DEBUG|GetbShowDebug) "BP_PC_Gameplay - Event Camera"))
    (:then_1
      (if (Pawn|IsLocalController)
        (CallFunction|EventPlayerControllerHUD)
        (CallFunction|EventPlayerControllerCamera)
        (CallFunction|EventPlayerControllerInteractInit)))))

(event Input|KeyboardEvents|DebugKey1
  (params (Key :type Key%20Structure :default "None") (ActionValue :type Input%20Action%20Value%20Structure))
  (:Pressed
    (CallFunction|EventDEBUGKillTargetUnit)))

(event Custom|EventPlayerControllerCamera
  (bind _returnvalue (PlayerController|LocalPlayerSubsystems|GetEnhancedInputLocalPlayerSubsystem))
  (Utilities|FlowControl|Sequence
    (:then_0
      (CallFunction|FuncShowDebugMessage (Variables|DEBUG|GetbShowDebug) "BP_PC_Gameplay - Event Camera"))
    (:then_1
      (Utilities|IsValid _returnvalue
        (:Is%20Valid
          (Input|AddMappingContext _returnvalue "/Game/PlayerList/Gameplay/Player/Input/IMC_Camera.IMC_Camera" 0 "(bIgnoreAllPressedKeysUntilRelease=True,bForceImmediately=False,bNotifyUserSettings=False)"))))
    (:then_2
      (Variables|Camera|GetAs%20BP_Pawn_Camera
        (:then)
        (:else
          (bind _asbp_pawn_camera (Utilities|Casting|CastToBP_Pawn_Camera (Pawn|GetControlledPawn)))
          (Variables|Camera|SetAs%20BP_Pawn_Camera _asbp_pawn_camera))))))

(event Input|EnhancedActionEvents|EnhancedInputActionIA_Camera_Move
  (params (ActionValue :type Boolean) (ElapsedSeconds :type Float%20%28double-precision%29) (TriggeredSeconds :type Float%20%28double-precision%29) (InputAction :type Input%20Action%20Object%20Reference :default "/Game/PlayerList/Gameplay/Player/Input/Actions/Camera/IA_Camera_Move.IA_Camera_Move"))
  (:Started
    (bind _as_bp_pawn_camera (Variables|Camera|GetAs%20BP_Pawn_Camera)
      (:then
        (Default|EventCameraMove _as_bp_pawn_camera))
      (:else))))

(event Input|EnhancedActionEvents|EnhancedInputActionIA_Camera_Rotate
  (params (ActionValue :type Boolean) (ElapsedSeconds :type Float%20%28double-precision%29) (TriggeredSeconds :type Float%20%28double-precision%29) (InputAction :type Input%20Action%20Object%20Reference :default "/Game/PlayerList/Gameplay/Player/Input/Actions/Camera/IA_Camera_Rotate.IA_Camera_Rotate"))
  (:Started
    (bind _as_bp_pawn_camera (Variables|Camera|GetAs%20BP_Pawn_Camera)
      (:then
        (Default|EventCameraRotate _as_bp_pawn_camera))
      (:else))))

(event Input|EnhancedActionEvents|EnhancedInputActionIA_Camera_Zoom
  (params (ActionValue :type Boolean) (ElapsedSeconds :type Float%20%28double-precision%29) (TriggeredSeconds :type Float%20%28double-precision%29) (InputAction :type Input%20Action%20Object%20Reference :default "/Game/PlayerList/Gameplay/Player/Input/Actions/Camera/IA_Camera_Zoom.IA_Camera_Zoom"))
  (:Started
    (bind _as_bp_pawn_camera (Variables|Camera|GetAs%20BP_Pawn_Camera)
      (:then
        (Default|EventCameraZoom _as_bp_pawn_camera))
      (:else))))

(event Input|EnhancedActionEvents|EnhancedInputActionIA_Camera_Focus
  (params (ActionValue :type Boolean) (ElapsedSeconds :type Float%20%28double-precision%29) (TriggeredSeconds :type Float%20%28double-precision%29) (InputAction :type Input%20Action%20Object%20Reference :default "/Game/PlayerList/Gameplay/Player/Input/Actions/Camera/IA_Camera_Focus.IA_Camera_Focus"))
  (:Started
    (bind _as_bp_pawn_camera (Variables|Camera|GetAs%20BP_Pawn_Camera)
      (:then
        (Default|EventCameraFocus _as_bp_pawn_camera))
      (:else))))

(event Custom|EventPlayerControllerInteractInit
  (bind _returnvalue (PlayerController|LocalPlayerSubsystems|GetEnhancedInputLocalPlayerSubsystem))
  (Utilities|FlowControl|Sequence
    (:then_0
      (CallFunction|FuncShowDebugMessage (Variables|DEBUG|GetbShowDebug) "BP_HUD_Gameplay - Event Interact"))
    (:then_1
      (Utilities|IsValid _returnvalue
        (:Is%20Valid
          (Input|AddMappingContext _returnvalue "/Game/PlayerList/Gameplay/Player/Input/IMC_Interact.IMC_Interact" 0 "(bIgnoreAllPressedKeysUntilRelease=True,bForceImmediately=False,bNotifyUserSettings=False)"))))
    (:then_2
      (Variables|Default|SetbShowMouseCursor true)
      (Variables|Default|SetbEnableMouseOverEvents true)
      (Variables|Default|SetCurrentClickTraceChannel "ECC_GameTraceChannel1"))))

(event Input|EnhancedActionEvents|EnhancedInputActionIA_Interact_Primary
  (params (ActionValue :type Boolean) (ElapsedSeconds :type Float%20%28double-precision%29) (TriggeredSeconds :type Float%20%28double-precision%29) (InputAction :type Input%20Action%20Object%20Reference :default "/Game/PlayerList/Gameplay/Player/Input/Actions/Interact/IA_Interact_Primary.IA_Interact_Primary"))
  (bind (_hit _hitactor) (CallFunction|GetActorUnderCursorbyChannel "TraceTypeQuery3"))
  (bind _returnvalue (PlayerController|LocalPlayerSubsystems|GetEnhancedInputLocalPlayerSubsystem))
  (bind _returnvalue_2 (PlayerController|LocalPlayerSubsystems|GetEnhancedInputLocalPlayerSubsystem))
  (:Started
    (bind _as_bp_actor_interact (Variables|Interact|GetAs%20BP_Actor_Interact)
      (:then
        (Class|BPIInteract|EndInteract(Message) _as_bp_actor_interact))
      (:else
        _))
    (if _hit
      (bind _output_get (Variables|Interact|SetAs%20BP_Actor_Interact _hitactor))
      (Class|BPIInteract|BeginInteract(Message) _output_get)
      (Development|PrintString "start ineract")
      (else
        (Utilities|IsValid _returnvalue_2
          (:Is%20Valid
            (Input|AddMappingContext _returnvalue_2 "/Game/PlayerList/Gameplay/Player/Input/IMC_Drag.IMC_Drag" 0 "(bIgnoreAllPressedKeysUntilRelease=True,bForceImmediately=False,bNotifyUserSettings=False)"))))))
  (:Completed
    (Utilities|IsValid _returnvalue
      (:Is%20Valid
        (Input|RemoveMappingContext _returnvalue "/Game/PlayerList/Gameplay/Player/Input/IMC_Drag.IMC_Drag" "(bIgnoreAllPressedKeysUntilRelease=True,bForceImmediately=False,bNotifyUserSettings=False)")))))

(event Input|EnhancedActionEvents|EnhancedInputActionIA_InteractSecondary
  (params (ActionValue :type Boolean) (ElapsedSeconds :type Float%20%28double-precision%29) (TriggeredSeconds :type Float%20%28double-precision%29) (InputAction :type Input%20Action%20Object%20Reference :default "/Game/PlayerList/Gameplay/Player/Input/Actions/Interact/IA_InteractSecondary.IA_InteractSecondary"))
  (:Started
    (bind _as_bp_actor_interact (Variables|Interact|GetAs%20BP_Actor_Interact)
      (:then
        (Class|BPIInteract|EndInteract(Message) _as_bp_actor_interact))
      (:else))))

(event Custom|EventPlayerControllerHUD
  (Utilities|FlowControl|Sequence
    (:then_0
      (CallFunction|FuncShowDebugMessage (Variables|DEBUG|GetbShowDebug) "BP_PC_Gameplay - Event HUD"))
    (:then_1
      (bind _asbp_hud_gameplay (Utilities|Casting|CastToBP_HUD_Gameplay (HUD|GetHUD)))
      (Variables|HUD|SetAs%20BP_HUD_Gameplay _asbp_hud_gameplay))))

(event Input|EnhancedActionEvents|EnhancedInputActionIA_Scoreboard
  (params (ActionValue :type Boolean) (ElapsedSeconds :type Float%20%28double-precision%29) (TriggeredSeconds :type Float%20%28double-precision%29) (InputAction :type Input%20Action%20Object%20Reference :default "/Game/PlayerList/Gameplay/Player/Input/Actions/Scoreboard/IA_Scoreboard.IA_Scoreboard"))
  (:Started
    (bind _as_bp_hud_gameplay (Variables|HUD|GetAs%20BP_HUD_Gameplay)
      (:then
        (Default|EventHUDWBPScoreboard _as_bp_hud_gameplay))
      (:else)))
  (:Canceled
    (bind _as_bp_hud_gameplay_2 (Variables|HUD|GetAs%20BP_HUD_Gameplay :!label _label)
      (:then
        (Default|EventHUDWBPScoreboard _as_bp_hud_gameplay_2))
      (:else)))
  (:Completed
    (goto _label)))

(event Custom|EventPlayerControllerUpdateUnit
  (params (Unit :type BP%20Character%20Unit%20Object%20Reference))
  (Utilities|FlowControl|Sequence
    (:then_0
      (CallFunction|FuncShowDebugMessage (Variables|DEBUG|GetbShowDebug) "BP_PC_Gameplay - Event Unit Update"))
    (:then_1
      (Variables|Unit|SetUnit Unit))))

(event EventSetLoadout
  (params (Loadout :type F%20Loadout%20Structure))
  (Variables|Loadout|SetLoadout Loadout))

(fn ConstructionScript)

(fn GetActorUnderCursorbyChannel
  (params (TraceChannel :type ETraceTypeQuery%20Enum :default "TraceTypeQuery1"))
  (bind _hitresult (Game|Player|GetHitResultUnderCursorbyChannel TraceChannel true))
  (bind (_bblockinghit _binitialoverlap _time _distance _location _impactpoint _normal _impactnormal _physmat _hitactor) (Collision|BreakHitResult _hitresult))
  (return _bblockinghit _hitactor))

(fn GetLoadout
  (return (Variables|Loadout|GetLoadout)))