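; Gameplay GameMode for the PlayerList project that handles team assignment, kill tracking and team scoring.
; On login it randomly sets the player state's team to Blue or Red, and on logout it removes the controller from its list.
; AddPlayerKill increments the indexed player's kills and the passed team's death counter on the GameState.
; FuncUpdateScore forwards score increases to the GameState, caching that reference on first use.
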(event Custom|AddPlayerKill
  (params (Team :type E_Team%20Enum :default "NewEnumerator0") (PlayerIndex :type Integer))
  (bind _asbp_ps_player_list (Utilities|Casting|CastToBP_PS_PlayerList (Variables|/Script/Engine.Controller|GetPlayerState (Utilities|Array|Get(acopy) (Variables|Default|GetAllPlayerControllers) PlayerIndex))))
  (Variables|/Game/PlayerList/Gameplay/Player/State/BP_PS_PlayerList.BP_PS_PlayerList_C|SetKills _asbp_ps_player_list (+ (Variables|/Game/PlayerList/Gameplay/Player/State/BP_PS_PlayerList.BP_PS_PlayerList_C|GetKills _asbp_ps_player_list) 1))
  ;[0.15 0.15 0.15 0.5] Add team score
  (switch Utilities|FlowControl|Switch|SwitchonE_Team Team
    (:NewEnumerator1
      (bind _as_bp_gs_gameplay (Variables|Default|GetAs%20BP_GS_Gameplay)
        (:then
          (Variables|/Game/PlayerList/Gameplay/System/BP_GS_Gameplay.BP_GS_Gameplay_C|SetBlueTeamDeaths _as_bp_gs_gameplay (+ (Variables|/Game/PlayerList/Gameplay/System/BP_GS_Gameplay.BP_GS_Gameplay_C|GetBlueTeamDeaths _as_bp_gs_gameplay) 1)))
        (:else)))
    (:NewEnumerator2
      (bind _as_bp_gs_gameplay_2 (Variables|Default|GetAs%20BP_GS_Gameplay)
        (:then
          (Variables|/Game/PlayerList/Gameplay/System/BP_GS_Gameplay.BP_GS_Gameplay_C|SetRedTeamDeaths _as_bp_gs_gameplay_2 (+ (Variables|/Game/PlayerList/Gameplay/System/BP_GS_Gameplay.BP_GS_Gameplay_C|GetRedTeamDeaths _as_bp_gs_gameplay_2) 1)))
        (:else)))))

(event EventBeginPlay
  (Utilities|FlowControl|Sequence
    (:then_0
      (CallFunction|FuncShowDebugMessage (Variables|DEBUG|GetbShowDebug) "BP_GM_Gameplay - Event Begin Play"))))

(event EventTick
  (params (DeltaSeconds :type Float%20%28single-precision%29)))

(event EventPostLogin
  (params (NewPlayer :type Player%20Controller%20Object%20Reference))
  (bind _asbp_ps_player_list (Utilities|Casting|CastToBP_PS_PlayerList (Variables|/Script/Engine.Controller|GetPlayerState NewPlayer)))
  (if (Math|Random|RandomBool)
    (Variables|/Game/PlayerList/Gameplay/Player/State/BP_PS_PlayerList.BP_PS_PlayerList_C|SetTeam _asbp_ps_player_list "NewEnumerator1")
    (else
      (Variables|/Game/PlayerList/Gameplay/Player/State/BP_PS_PlayerList.BP_PS_PlayerList_C|SetTeam _asbp_ps_player_list "NewEnumerator2"))))

(event EventOnLogout
  (params (ExitingController :type Controller%20Object%20Reference))
  (bind _asplayer_controller (Utilities|Casting|CastToPlayerController ExitingController))
  (Utilities|Array|RemoveItem (Variables|Default|GetAllPlayerControllers) _asplayer_controller))

(event EventOnSwapPlayerControllers
  (params (OldPC :type Player%20Controller%20Object%20Reference) (NewPC :type Player%20Controller%20Object%20Reference)))

(fn ConstructionScript)

(fn FuncUpdateScore
  (params (Team :type E_Team%20Enum :default "NewEnumerator0"))
  (Variables|Default|GetAs%20BP_GS_Gameplay
    (:then
      _)
    (:else
      (bind _asbp_gs_gameplay (Utilities|Casting|CastToBP_GS_Gameplay (Game|GetGameState)))
      (Variables|Default|SetAs%20BP_GS_Gameplay _asbp_gs_gameplay)))
  (Default|FuncIncreaseTeamScore (Variables|Default|GetAs%20BP_GS_Gameplay) Team))