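; Gameplay GameState that tracks the connected player list and the Blue and Red team scores.
; UpdatePlayerList copies PlayerArray into AllPlayerStates, and Func_IncreaseTeamScore adds one point to the given team.
; All three variables use RepNotify, whose OnRep functions broadcast the OnUpdateConnectedPlayer and OnUpdateTeamScore dispatchers so listeners can react to changes without polling.
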(event Custom|UpdatePlayerList
  (Variables|Default|SetAllPlayerStates (Variables|Default|GetPlayerArray)))

(event EventBeginPlay)

(event EventTick
  (params (DeltaSeconds :type Float%20%28single-precision%29)))

(fn ConstructionScript)

(fn FuncIncreaseTeamScore
  (params (Team :type E_Team%20Enum :default "NewEnumerator0"))
  (switch Utilities|FlowControl|Switch|SwitchonE_Team Team
    (:NewEnumerator1
      (Variables|Default|SetBlueTeamScore (+ (Variables|Default|GetBlueTeamScore) 1)))
    (:NewEnumerator2
      (Variables|Default|SetRedTeamScore (+ (Variables|Default|GetRedTeamScore) 1)))))

(fn OnRepAllPlayerStates
  (Default|CallOnUpdateConnectedPlayer (Variables|Default|GetAllPlayerStates)))

(fn OnRepBlueTeamScore
  (Default|CallOnUpdateTeamScore (Variables|Default|GetBlueTeamScore) (Variables|Default|GetRedTeamScore)))

(fn OnRepRedTeamScore
  (Default|CallOnUpdateTeamScore (Variables|Default|GetBlueTeamScore) (Variables|Default|GetRedTeamScore)))