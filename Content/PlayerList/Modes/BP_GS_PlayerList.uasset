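; Game State for player-list modes that replicates the player roster and Blue and Red team scores.
; UpdatePlayerList copies PlayerArray into AllPlayerStates, whose RepNotify finds every WB_HUD_Scoreboard widget and refreshes it.
; RepNotifies on either team score call the OnUpdateTeamScore dispatcher with both current scores.
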(event Custom|UpdatePlayerList
  (Variables|Default|SetAllPlayerStates (Variables|Default|GetPlayerArray)))

(event EventBeginPlay)

(event EventTick
  (params (DeltaSeconds :type Float%20%28single-precision%29)))

(fn ConstructionScript)

(fn OnRepAllPlayerStates
  (bind _foundwidgets (Widget|GetAllWidgetsOfClass "/Game/PlayerList/UI/HUD/Scoreboard/WB_HUD_Scoreboard.WB_HUD_Scoreboard_C" false))
  (for _array_element _foundwidgets
    (Default|UpdateWBScoreboard _array_element)))

(fn OnRepBlueTeamScore
  (Default|CallOnUpdateTeamScore (Variables|Default|GetBlueTeamScore) (Variables|Default|GetRedTeamScore)))

(fn OnRepRedTeamScore
  (Default|CallOnUpdateTeamScore (Variables|Default|GetBlueTeamScore) (Variables|Default|GetRedTeamScore)))