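; Game mode for the player list system that tracks connected controllers, assigns teams and handles kills and kicks.
; Logins alternate Blue and Red by controller count parity.
; Joins and leaves update the controller array, then call the game state's list refresh after a short delay for replication.
; Kills increment player state and game state team scores; kicks go through the player controller's owning-client call, both addressed by array index.
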(event Custom|UpdateConnectedPlayers
  ;[0.15 0.15 0.15 0.5] Allow time for replication
  (Utilities|FlowControl|Delay 0.3)
  (bind _asbp_gs_player_list (Utilities|Casting|CastToBP_GS_PlayerList (Game|GetGameState)))
  (Default|UpdatePlayerList _asbp_gs_player_list))

(event Custom|AddPlayerKill
  (params (Team :type E_Team%20Enum :default "NewEnumerator0") (PlayerIndex :type Integer))
  (bind _asbp_ps_player_list (Utilities|Casting|CastToBP_PS_PlayerList (Variables|/Script/Engine.Controller|GetPlayerState (Utilities|Array|Get(acopy) (Variables|Default|GetAllPlayerControllers) PlayerIndex))))
  (Variables|/Game/PlayerList/Player/BP_PS_PlayerList.BP_PS_PlayerList_C|SetKills _asbp_ps_player_list (+ (Variables|/Game/PlayerList/Player/BP_PS_PlayerList.BP_PS_PlayerList_C|GetKills _asbp_ps_player_list) 1))
  ;[0.15 0.15 0.15 0.5] Add team score
  (switch Utilities|FlowControl|Switch|SwitchonE_Team Team
    (:NewEnumerator1
      (bind _as_bp_gs_player_list (Variables|Default|GetAs%20BP%20GS%20Player%20List)
        (:then
          (Variables|/Game/PlayerList/Modes/BP_GS_PlayerList.BP_GS_PlayerList_C|SetBlueTeamScore _as_bp_gs_player_list (+ (Variables|/Game/PlayerList/Modes/BP_GS_PlayerList.BP_GS_PlayerList_C|GetBlueTeamScore _as_bp_gs_player_list) 1)))
        (:else)))
    (:NewEnumerator2
      (bind _as_bp_gs_player_list_2 (Variables|Default|GetAs%20BP%20GS%20Player%20List)
        (:then
          (Variables|/Game/PlayerList/Modes/BP_GS_PlayerList.BP_GS_PlayerList_C|SetRedTeamScore _as_bp_gs_player_list_2 (+ (Variables|/Game/PlayerList/Modes/BP_GS_PlayerList.BP_GS_PlayerList_C|GetRedTeamScore _as_bp_gs_player_list_2) 1)))
        (:else)))))

(event EventBeginPlay
  (bind _asbp_gs_player_list (Utilities|Casting|CastToBP_GS_PlayerList (Game|GetGameState)))
  (Variables|Default|SetAs%20BP%20GS%20Player%20List _asbp_gs_player_list))

(event EventTick
  (params (DeltaSeconds :type Float%20%28single-precision%29)))

(event EventPostLogin
  (params (NewPlayer :type Player%20Controller%20Object%20Reference))
  (Utilities|Array|Add (Variables|Default|GetAllPlayerControllers) NewPlayer)
  (CallFunction|UpdateConnectedPlayers)
  (bind _asbp_ps_player_list (Utilities|Casting|CastToBP_PS_PlayerList (Variables|/Script/Engine.Controller|GetPlayerState NewPlayer)))
  (if (> (Math|Integer|%(Integer) (Utilities|Array|Length (Variables|Default|GetAllPlayerControllers)) 2) 0)
    (Variables|/Game/PlayerList/Player/BP_PS_PlayerList.BP_PS_PlayerList_C|SetTeam _asbp_ps_player_list "NewEnumerator1")
    (else
      (Variables|/Game/PlayerList/Player/BP_PS_PlayerList.BP_PS_PlayerList_C|SetTeam _asbp_ps_player_list "NewEnumerator2"))))

(event EventOnLogout
  (params (ExitingController :type Controller%20Object%20Reference))
  (bind _asplayer_controller (Utilities|Casting|CastToPlayerController ExitingController))
  (Utilities|Array|RemoveItem (Variables|Default|GetAllPlayerControllers) _asplayer_controller)
  (CallFunction|UpdateConnectedPlayers))

(fn ConstructionScript)

(fn KickPlayer
  (params (PlayerID :type Integer))
  (bind _asbp_pc_player_list (Utilities|Casting|CastToBP_PC_PlayerList (Utilities|Array|Get(acopy) (Variables|Default|GetAllPlayerControllers) PlayerID)))
  (Default|OwningClientKickPlayer _asbp_pc_player_list))